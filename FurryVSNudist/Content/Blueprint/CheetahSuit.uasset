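; CheetahSuit is a power-up pickup that turns the player into a cheetah.
; When an FCharacter_BP overlaps it, player 0's character gets the Gepard skeletal mesh and new walk speed and jump velocity, then the pickup destroys itself.
; While idle, Tick spins it and plays a timeline that feeds local offsets to move it.
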(event `self.ReceiveActorBeginOverlap`
  (params (OtherActor :type "Actor Object Reference"))
  (bind _returnvalue (`GameplayStatics.GetPlayerCharacter` 0))
  (bind _charactermovement (`Character.CharacterMovement` _returnvalue))
  ;[1 1 1] Bunny Suit
  (cast `/Game/Blueprint/FCharacter_BP` OtherActor)
  (`ActorComponent.K2_DestroyComponent` (`self.StaticMesh`))
  (`ActorComponent.K2_DestroyComponent` (`self.Collision`))
  (`KismetSystemLibrary.PrintString` "Put on Cheetah Suit")
  (`SkinnedMeshComponent.SetSkinnedAssetAndUpdate` (`Character.Mesh` _returnvalue) "/Game/Meshes/Characters/Gepard.Gepard" true)
  (set `CharacterMovementComponent.MaxWalkSpeed` 1000.0 _charactermovement)
  (set `CharacterMovementComponent.JumpZVelocity` 400.0 _charactermovement)
  (`self.K2_DestroyActor`))

(event `self.ReceiveTick`
  (params (DeltaSeconds :type "Float (single-precision)"))
  ;[1 1 1] Power up idle
  (`self.K2_AddActorLocalRotation` (struct :`Yaw` 1.0))
  (bind (_direction _movement) (`Timeline|Timeline_0`)
    (:`Update`
      (`self.K2_AddActorLocalOffset` _movement))))

(fn `UserConstructionScript`)