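; Base player controller for cursor-aimed character control, with the mouse cursor shown from BeginPlay.
; Each tick it traces under the cursor on the Visibility channel and yaws the controlled pawn to face the hit location.
; Up and Right axes move the pawn along the camera manager's up and right vectors, making movement screen-relative rather than facing-relative.
; The Jump action makes the pawn jump if it is a Character.
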(event `self.ReceiveBeginPlay`
  ;[1 1 1] Show Mouse Cursor
  (set `self.bShowMouseCursor` true))

(event `self.ReceiveTick`
  (params (DeltaSeconds :type "Float (single-precision)"))
  ;[1 1 1] Camera
  (`self.ProcessMouse`))

(event `ProcessMouse`
  (bind (_hitresult _returnvalue) (`self.GetHitResultUnderCursorByChannel` "TraceTypeQuery1"))
  (bind _returnvalue_2 (`self.K2_GetPawn`))
  (bind (_returnvalue_roll _returnvalue_pitch _returnvalue_yaw) (`KismetMathLibrary.BreakRotator` (`KismetMathLibrary.Conv_VectorToRotator` (`KismetMathLibrary.GetDirectionUnitVector` (`self.K2_GetActorLocation` _returnvalue_2) (`.Location` (`GameplayStatics.BreakHitResult` _hitresult))))))
  ;[1 1 1] Camera
  (`/Engine/EditorBlueprintResources/StandardMacros.IsValid` (`self.K2_GetPawn`)
    (:`Is Valid`
      (if _returnvalue
        (`self.K2_SetActorRotation` _returnvalue_2 (`KismetMathLibrary.MakeRotator` 0.0 0.0 _returnvalue_yaw) false)))))

(event `InputAxis|Up`
  (params (AxisValue :type "Float (single-precision)"))
  (bind _returnvalue (`self.K2_GetPawn`))
  ;[1 1 1] Movement
  (`/Engine/EditorBlueprintResources/StandardMacros.IsValid` _returnvalue
    (:`Is Valid`
      (`Pawn.AddMovementInput` _returnvalue (`SceneComponent.GetUpVector` (`PlayerCameraManager.TransformComponent` (`self.PlayerCameraManager`))) AxisValue false))))

(event `InputAxis|Right`
  (params (AxisValue :type "Float (single-precision)"))
  (bind _returnvalue (`self.K2_GetPawn`))
  ;[1 1 1] Movement
  (`/Engine/EditorBlueprintResources/StandardMacros.IsValid` _returnvalue
    (:`Is Valid`
      (`Pawn.AddMovementInput` _returnvalue (`SceneComponent.GetRightVector` (`PlayerCameraManager.TransformComponent` (`self.PlayerCameraManager`))) AxisValue false))))

(event `InputAction|Jump`
  (params (Key :type "Key Structure"))
  ;[1 1 1] Movement
  (:`Pressed`
    (bind _ascharacter (cast `Character` (`self.K2_GetPawn`)))
    (`Character.Jump` _ascharacter)))

(fn `UserConstructionScript`)